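; PatrolingEnemy_BP is an enemy Blueprint that exposes AI controller movement commands; the patrol route logic is not in this graph.
; MovetoLocation cancels any current move, then sends the controller to the given location with a small acceptance radius and no strafing or partial paths.
; StopMoving halts movement and prints a debug string.
; Tick sets ReachedDestination whenever the move status is Idle and prints it every frame.
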(event EventTick
  (params (DeltaSeconds :type Float%20%28single-precision%29))
  (bind _output_get (Variables|Default|SetbReachedDestination (Utilities|Enum|Equal(Enum) (Class|AIController|GetMoveStatus (AI|GetAIController self)) "Idle")))
  (Development|PrintString (Utilities|String|ToString(Boolean) _output_get)))

(event EventMovetoLocation
  (params (Location :type Vector :default "0, 0, 0"))
  (bind _self self)
  (bind _returnvalue (AI|GetAIController _self))
  (AI|Navigation|StopMovement _returnvalue)
  (AI|Navigation|MovetoLocation _returnvalue Location 6.0 true true false false 0 false))

(event EventStopMoving
  (AI|Navigation|StopMovement (AI|GetAIController self))
  (Development|PrintString ":v"))

(fn ConstructionScript)