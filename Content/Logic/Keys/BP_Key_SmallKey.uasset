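; BP_Key_SmallKey is a small key actor built from three cube components and a cylinder.
; It overrides UpdateFinishedVisuals, running the parent logic first, then hiding Cube along with its child components and turning off collision on all four components.
; BeginPlay, overlap, Tick and the construction script add no logic.
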(event EventBeginPlay)

(event Collision|EventActorBeginOverlap
  (params (OtherActor :type Actor%20Object%20Reference)))

(event EventTick
  (params (DeltaSeconds :type Float%20%28single-precision%29)))

(event EventUpdateFinishedVisuals
  (|CallParentFunction)
  (Rendering|SetVisibility (Variables|Default|GetCube) false true)
  (Collision|SetCollisionEnabled (Variables|Default|GetCube) "NoCollision")
  (Collision|SetCollisionEnabled (Variables|Default|GetCube1) "NoCollision")
  (Collision|SetCollisionEnabled (Variables|Default|GetCube2) "NoCollision")
  (Collision|SetCollisionEnabled (Variables|Default|GetCylinder) "NoCollision"))

(fn ConstructionScript)