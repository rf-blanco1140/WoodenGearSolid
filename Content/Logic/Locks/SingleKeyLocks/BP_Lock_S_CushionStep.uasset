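; BP_Lock_S_CushionStep is a single-key lock that reveals a solid step cube when its finished visuals update.
; An ActivationRange overlap caches the player pawn, and the construction script starts the Cube with collision disabled.
; UpdateFinishedVisuals runs the parent logic, moves the cached player to PullingPosition, then makes the Cube visible with query and physics collision.
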(event OnComponentBeginOverlap(ActivationRange)
  (params (OverlappedComponent :type Primitive%20Component%20Object%20Reference) (OtherActor :type Actor%20Object%20Reference) (OtherComp :type Primitive%20Component%20Object%20Reference) (OtherBodyIndex :type Integer) (bFromSweep :type Boolean) (SweepResult :type Hit%20Result%20Structure%20%28by%20ref%29))
  (if (== OtherActor (Game|Player|GetPlayerPawn 0))
    (Variables|Default|SetPlayerRef OtherActor)))

(event EventBeginPlay
  (|CallParentFunction) ; This node is disabled and will not be called.\nDrag off pins to build functionality.
)

(event Collision|EventActorBeginOverlap
  (params (OtherActor :type Actor%20Object%20Reference))
  (|CallParentFunction OtherActor) ; This node is disabled and will not be called.\nDrag off pins to build functionality.
)

(event EventTick
  (params (DeltaSeconds :type Float%20%28single-precision%29))
  (|CallParentFunction DeltaSeconds) ; This node is disabled and will not be called.\nDrag off pins to build functionality.
)

(event EventUpdateFinishedVisuals
  (bind _cube (Variables|Default|GetCube))
  (|CallParentFunction)
  (Transformation|SetActorLocation (Variables|Default|GetPlayerRef) (Transformation|GetWorldLocation (Variables|Default|GetPullingPosition)) false false)
  (Rendering|SetVisibility _cube true true)
  (Collision|SetCollisionEnabled _cube "QueryAndPhysics"))

(fn ConstructionScript
  (|CallParentFunction)
  (Collision|SetCollisionEnabled (Variables|Default|GetCube) "NoCollision"))