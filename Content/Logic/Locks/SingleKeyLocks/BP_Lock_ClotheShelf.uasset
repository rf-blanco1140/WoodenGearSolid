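; Clothes-shelf lock Blueprint that reveals an open shelf when the lock's finished visuals are applied.
; Construction hides OpenShelf1 with its children and disables collision on both open-shelf components.
; An ActivationRange overlap caches the player pawn as PlayerRef.
; UpdateFinishedVisuals calls the parent, moves the player to PullingPosition without sweeping, then shows OpenShelf1 and enables collision on both shelves.
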(event OnComponentBeginOverlap(ActivationRange)
  (params (OverlappedComponent :type Primitive%20Component%20Object%20Reference) (OtherActor :type Actor%20Object%20Reference) (OtherComp :type Primitive%20Component%20Object%20Reference) (OtherBodyIndex :type Integer) (bFromSweep :type Boolean) (SweepResult :type Hit%20Result%20Structure%20%28by%20ref%29))
  (if (== OtherActor (Game|Player|GetPlayerPawn 0))
    (Variables|Default|SetPlayerRef OtherActor)))

(event EventBeginPlay)

(event Collision|EventActorBeginOverlap
  (params (OtherActor :type Actor%20Object%20Reference)))

(event EventTick
  (params (DeltaSeconds :type Float%20%28single-precision%29)))

(event EventUpdateFinishedVisuals
  (bind _openshelf_1 (Variables|Default|GetOpenShelf_1))
  (|CallParentFunction)
  (Transformation|SetActorLocation (Variables|Default|GetPlayerRef) (Transformation|GetWorldLocation (Variables|Default|GetPullingPosition)) false false)
  (Rendering|SetVisibility _openshelf_1 true true)
  (Collision|SetCollisionEnabled _openshelf_1 "QueryAndPhysics")
  (Collision|SetCollisionEnabled (Variables|Default|GetOpenShelf_2) "QueryAndPhysics"))

(fn ConstructionScript
  (bind _openshelf_1 (Variables|Default|GetOpenShelf_1))
  (Rendering|SetVisibility _openshelf_1 false true)
  (Collision|SetCollisionEnabled _openshelf_1 "NoCollision")
  (Collision|SetCollisionEnabled (Variables|Default|GetOpenShelf_2) "NoCollision"))