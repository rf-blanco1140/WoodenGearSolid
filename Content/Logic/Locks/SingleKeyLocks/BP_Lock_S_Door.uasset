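; BP_Lock_S_Door is a single-key lock variant for a door, extending a parent lock Blueprint.
; When the finished visuals update, it rotates RotationPoint a quarter turn and toggles the Lock component's visibility.
; The player entering ActivationRange starts a hovering billboard, using a FlipFlop that alternately plays and reverses a timeline-driven position lerp.
; The timeline's Finished output re-triggers the loop, and leaving the range stops it in place.
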(event OnComponentBeginOverlap(ActivationRange)
  (params (OverlappedComponent :type Primitive%20Component%20Object%20Reference) (OtherActor :type Actor%20Object%20Reference) (OtherComp :type Primitive%20Component%20Object%20Reference) (OtherBodyIndex :type Integer) (bFromSweep :type Boolean) (SweepResult :type Hit%20Result%20Structure%20%28by%20ref%29))
  ;[1 1 1] Hovering Billboard On/OFF
  (if (== OtherActor (Game|Player|GetPlayerPawn 0))
    (Utilities|FlowControl|FlipFlop
      (:A
        (bind _lerp_0_1 (Timeline|Timeline_0 Play)
          (:Update
            (Transformation|SetRelativeLocation (Variables|Default|GetBillboard) (Math|Vector|Lerp(Vector) "100.000000,0.000000,0.000000" "100.000000, 0,50.000000" _lerp_0_1) true false))
          (:Finished
            (CallFunction|PlayLerp))))
      (:B
        (Timeline|Timeline_0 Reverse)))))

(event OnComponentEndOverlap(ActivationRange)
  (params (OverlappedComponent :type Primitive%20Component%20Object%20Reference) (OtherActor :type Actor%20Object%20Reference) (OtherComp :type Primitive%20Component%20Object%20Reference) (OtherBodyIndex :type Integer))
  ;[1 1 1] Hovering Billboard On/OFF
  (if (== OtherActor (Game|Player|GetPlayerPawn 0))
    (bind _lerp_0_1 (Timeline|Timeline_0 Stop)
      (:Update
        (Transformation|SetRelativeLocation (Variables|Default|GetBillboard) (Math|Vector|Lerp(Vector) "100.000000,0.000000,0.000000" "100.000000, 0,50.000000" _lerp_0_1) true false))
      (:Finished
        (CallFunction|PlayLerp)))))

(event Custom|PlayLerp
  ;[1 1 1] Hovering Billboard On/OFF
  (Utilities|FlowControl|FlipFlop
    (:A
      (bind _lerp_0_1 (Timeline|Timeline_0 Play)
        (:Update
          (Transformation|SetRelativeLocation (Variables|Default|GetBillboard) (Math|Vector|Lerp(Vector) "100.000000,0.000000,0.000000" "100.000000, 0,50.000000" _lerp_0_1) true false))
        (:Finished
          (CallFunction|PlayLerp))))
    (:B
      (Timeline|Timeline_0 Reverse))))

(event EventBeginPlay
  (|CallParentFunction) ; This node is disabled and will not be called.\nDrag off pins to build functionality.
)

(event Collision|EventActorBeginOverlap
  (params (OtherActor :type Actor%20Object%20Reference))
  (|CallParentFunction OtherActor) ; This node is disabled and will not be called.\nDrag off pins to build functionality.
)

(event EventTick
  (params (DeltaSeconds :type Float%20%28single-precision%29))
  (|CallParentFunction DeltaSeconds) ; This node is disabled and will not be called.\nDrag off pins to build functionality.
)

(event EventUpdateFinishedVisuals
  (|CallParentFunction)
  (Transformation|SetRelativeRotation (Variables|Default|GetRotationPoint) "0,-90.000000, 0" false false)
  (Rendering|ToggleVisibility (Variables|Default|GetLock) false))

(fn ConstructionScript
  (|CallParentFunction))