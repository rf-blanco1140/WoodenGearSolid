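; BP_Lock_S_SmallStaircase is a single-key lock variant that reveals a small staircase when its finished visuals update.
; The construction script calls the parent, then disables collision on two cube components.
; UpdateFinishedVisuals calls the parent, then toggles both cubes' visibility, propagating to children, and enables query and physics collision.
; Visibility is toggled rather than set, so the result depends on the cubes' current state.
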(event EventBeginPlay
  (|CallParentFunction) ; This node is disabled and will not be called.\nDrag off pins to build functionality.
)

(event Collision|EventActorBeginOverlap
  (params (OtherActor :type Actor%20Object%20Reference))
  (|CallParentFunction OtherActor) ; This node is disabled and will not be called.\nDrag off pins to build functionality.
)

(event EventTick
  (params (DeltaSeconds :type Float%20%28single-precision%29))
  (|CallParentFunction DeltaSeconds) ; This node is disabled and will not be called.\nDrag off pins to build functionality.
)

(event EventUpdateFinishedVisuals
  (bind _cube (Variables|Default|GetCube))
  (bind _cube1 (Variables|Default|GetCube1))
  (|CallParentFunction)
  (Rendering|ToggleVisibility _cube true)
  (Collision|SetCollisionEnabled _cube "QueryAndPhysics")
  (Rendering|ToggleVisibility _cube1 true)
  (Collision|SetCollisionEnabled _cube1 "QueryAndPhysics"))

(fn ConstructionScript
  (|CallParentFunction)
  (Collision|SetCollisionEnabled (Variables|Default|GetCube) "NoCollision")
  (Collision|SetCollisionEnabled (Variables|Default|GetCube1) "NoCollision"))