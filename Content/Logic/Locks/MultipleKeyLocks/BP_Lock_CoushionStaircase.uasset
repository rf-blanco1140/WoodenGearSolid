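; Lock Blueprint for a cushion staircase that becomes solid when the lock's finished visuals update.
; The construction script disables collision on three cube components.
; UpdateFinishedVisuals calls the parent, shows Cube and Cube1, then enables query and physics collision on all three cubes.
; Cube2's visibility call is disconnected, so this event leaves its visibility unchanged.
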(event EventBeginPlay
  (|CallParentFunction) ; This node is disabled and will not be called.\nDrag off pins to build functionality.
)

(event Collision|EventActorBeginOverlap
  (params (OtherActor :type Actor%20Object%20Reference))
  (|CallParentFunction OtherActor) ; This node is disabled and will not be called.\nDrag off pins to build functionality.
)

(event EventTick
  (params (DeltaSeconds :type Float%20%28single-precision%29))
  (|CallParentFunction DeltaSeconds))

(event EventUpdateFinishedVisuals
  (bind _cube (Variables|Default|GetCube))
  (bind _cube1 (Variables|Default|GetCube1))
  (|CallParentFunction)
  (Rendering|SetVisibility _cube true true)
  (Collision|SetCollisionEnabled _cube "QueryAndPhysics")
  (Rendering|SetVisibility _cube1 true true)
  (Collision|SetCollisionEnabled _cube1 "QueryAndPhysics")
  (Collision|SetCollisionEnabled (Variables|Default|GetCube2) "QueryAndPhysics"))

(fn ConstructionScript
  (|CallParentFunction)
  (Collision|SetCollisionEnabled (Variables|Default|GetCube) "NoCollision")
  (Collision|SetCollisionEnabled (Variables|Default|GetCube1) "NoCollision")
  (Collision|SetCollisionEnabled (Variables|Default|GetCube2) "NoCollision"))