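; KidController_BP is a controller that owns the pause menu and handles pausing the game.
; On possess it creates WBP_PauseMenu, adds it to the viewport, and immediately calls ToggleGame; the Pause input calls the same function and prints a debug string.
; ToggleGame flips IsPaused, shows or collapses the menu, sets the game's paused state, and restores game-only input when unpausing.
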(event EventPossess
  (params (PossessedPawn :type Pawn%20Object%20Reference))
  (bind _returnvalue (UserInterface|CreateWidget "/Game/Logic/UI/WBP_PauseMenu.WBP_PauseMenu_C" self))
  (bind _output_get (Variables|Default|SetPauseMenu _returnvalue))
  (UserInterface|Viewport|AddtoViewport _output_get 0)
  (CallFunction|ToggleGame))

(event Input|ActionEvents|InputActionPause
  (params (Key :type Key%20Structure))
  (:Pressed
    (CallFunction|ToggleGame)
    (Development|PrintString "Hello")))

(fn ConstructionScript)

(fn ToggleGame
  (bind _pausemenu (Variables|Default|GetPauseMenu))
  (bind _output_get (Variables|Default|SetbIsPaused (not (Variables|Default|GetbIsPaused))))
  (if _output_get
    (Widget|SetVisibility _pausemenu "Visible")
    (else
      (Widget|SetVisibility _pausemenu "Collapsed")))
  (Game|SetGamePaused (Variables|Default|GetbIsPaused))
  (if (not (Variables|Default|GetbIsPaused))
    (Input|SetInputModeGameOnly self)))