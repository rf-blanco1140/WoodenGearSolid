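; BP_Drawer is an interactable drawer that can be opened once, only with the key matching its KeyCode.
; It creates a pop-up widget holding a self-reference, shown while closed and removed on hide.
; ShowPopUp caches whether it can open, while interaction re-checks the obtained keys.
; Opening involves no animation: it reveals Cube1 and enables collision on Cube1 and Cube2, which the Construction Script hides or disables.
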(event EventHidePopUp
  (Widget|RemovefromParent (Variables|Default|GetPopUp_Widget)))

(event EventShowPopUp
  (params (Obtained%20Keys :type Array%20of%20Booleans))
  ;[1 1 1] Shows pop-up
  (if (not (Variables|Default|GetIsOpen))
    (Variables|Default|SetCanBeOpened (Utilities|Array|Get(acopy) Obtained%20Keys (Variables|Default|GetKey%20Code)))
    (UserInterface|Viewport|AddtoViewport (Variables|Default|GetPopUp_Widget) 0)))

(event EventBeginPlay
  ;[1 1 1] Creates UI Widget and sets reference of self inside the Widget
  (bind _returnvalue (UserInterface|CreateWidget "/Game/BP/BP_W_PopUp.BP_W_PopUp_C"))
  (bind _output_get (Variables|Default|SetPopUp_Widget _returnvalue))
  (Variables|/Game/BP/BP_W_PopUp.BP_W_PopUp_C|SetInteractableRef _output_get self))

(event EventInteractwithObject
  (if (not (Variables|Default|GetIsOpen))
    (if (Utilities|Array|Get(acopy) (Variables|Default|GetObtained%20Keys) (Variables|Default|GetKey%20Code))
      (Variables|Default|SetIsOpen true)
      (Rendering|SetVisibility (Variables|Default|GetCube1) true true)
      (Collision|SetCollisionEnabled (Variables|Default|GetCube1) "QueryAndPhysics")
      (Collision|SetCollisionEnabled (Variables|Default|GetCube2) "QueryAndPhysics"))))

(fn ConstructionScript
  (Rendering|SetVisibility (Variables|Default|GetCube1) false true)
  (Collision|SetCollisionEnabled (Variables|Default|GetCube1) "NoCollision")
  (Collision|SetCollisionEnabled (Variables|Default|GetCube2) "NoCollision"))