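; Bed-bound guardian that watches for the player and prints "GO TO SLEEP!!!" on detection.
; While not suspecting, a Tick timer periodically flips the mesh between two sides, toggling the Box1 detection volume off and on.
; An overlapping standing player is caught immediately, while a crouching one shows the Cone and starts suspicion, caught once DetectionTimer passes its threshold.
; Leaving the box clears suspicion and hides the Cone, but DetectionTimer never resets.
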(event OnComponentBeginOverlap(Box1)
  (params (OverlappedComponent :type Primitive%20Component%20Object%20Reference) (OtherActor :type Actor%20Object%20Reference) (OtherComp :type Primitive%20Component%20Object%20Reference) (OtherBodyIndex :type Integer) (bFromSweep :type Boolean) (SweepResult :type Hit%20Result%20Structure%20%28by%20ref%29))
  ;[1 1 1] Detect Player
  (if (Utilities|DoesObjectImplementInterface OtherActor "/Game/BP/BP_I_Player.BP_I_Player_C")
    (if (AI|Components|NavMovement|IsCrouching (Variables|/Script/Engine.Character|GetCharacterMovement (Variables|Default|GetPlayerCharacter)))
      (Rendering|SetVisibility (Variables|Default|GetCone) true true)
      (Variables|Default|SetIsSuspecting true)
      (else
        (Development|PrintString "GO TO SLEEP!!!" true true "(R=1.000000,G=0.000000,B=0.016462,A=1.000000)")))))

(event OnComponentEndOverlap(Box1)
  (params (OverlappedComponent :type Primitive%20Component%20Object%20Reference) (OtherActor :type Actor%20Object%20Reference) (OtherComp :type Primitive%20Component%20Object%20Reference) (OtherBodyIndex :type Integer))
  ;[1 1 1] Forgetting the player
  (if (Utilities|DoesObjectImplementInterface OtherActor "/Game/BP/BP_I_Player.BP_I_Player_C")
    (Variables|Default|SetIsSuspecting false)
    (Rendering|SetVisibility (Variables|Default|GetCone) false true)))

(event EventBeginPlay
  ;[1 1 1] Initialize Player Character Reference
  (bind _asbp_third_person_character (Utilities|Casting|CastToBP_ThirdPersonCharacter (Game|Player|GetPlayerPawn 0)))
  (Variables|Default|SetPlayerCharacter _asbp_third_person_character))

(event EventTick
  (params (DeltaSeconds :type Float%20%28single-precision%29))
  (bind _guardianmesh (Variables|Default|GetGuardianMesh))
  (bind _box1 (Variables|Default|GetBox1))
  (if (Variables|Default|GetIsSuspecting)
    ;[1 1 1] Find Crouching Player
    (bind _output_get (Variables|Default|SetDetectionTimer (+ (Variables|Default|GetDetectionTimer) DeltaSeconds)))
    (if (> _output_get 3.0)
      (Development|PrintString "GO TO SLEEP!!!" true true "(R=1.000000,G=0.000000,B=0.016462,A=1.000000)"))
    (else
      ;[1 1 1] Rotate in Bed
      (bind _output_get_2 (Variables|Default|SetRotation%20Timer (+ DeltaSeconds (Variables|Default|GetRotation%20Timer))))
      (if (> _output_get_2 3.0)
        (Variables|Default|SetRotation%20Timer 0.0)
        (Utilities|FlowControl|FlipFlop
          (:A
            (Transformation|SetRelativeRotation _guardianmesh "-90.000000,0.000000,-90.000000" false false)
            (Collision|SetCollisionEnabled _box1 "NoCollision"))
          (:B
            (Transformation|SetRelativeRotation _guardianmesh "90.000000,0.0,-90.000000" false false)
            (Collision|SetCollisionEnabled _box1 "QueryOnly")))))))

(fn ConstructionScript
  (Rendering|SetVisibility (Variables|Default|GetCone) false true))